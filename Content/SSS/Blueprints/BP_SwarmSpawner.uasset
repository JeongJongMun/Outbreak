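; Swarm spawner that spawns enemies around the player from data-table settings and the current wave's entries.
; A timed loop rolls chance and count per enemy type, stopping at the enemy cap; EnemyDestroyed decrements the count without restarting it.
; FindRandomLocation sweeps spheres vertically around a distance ring, with optional tag filtering, closest-height choice and above/below spawning.
; It picks randomly among navmesh-validated points, with optional debug drawing.
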(event Custom|SpawnEnemiesLoop
  ;[0 0 0 0.5] Main System Spawn Loop
  ;;[0.15 0.15 0.15 0.5] Main Spawn Function
  (CallFunction|SpawnEnemies)
  ;;[0.15 0.15 0.15 0.5] Check for Enemy Limit before trying to Spawn more
  (if (< (Variables|VariableData|GetSpawnedEnemies) (Utilities|Struct|BreakSSS_S_Settings (Variables|StaticData|GetSettings)))
    ;;[0.15 0.15 0.15 0.5] Interval between Spawn Calls
    (Utilities|FlowControl|Delay (Utilities|Struct|BreakSSS_S_Settings (Variables|StaticData|GetSettings)))
    ;;[0.15 0.15 0.15 0.5] Loop Call
    (CallFunction|SpawnEnemiesLoop)))

(event Custom|EnemyDestroyed
  ;[0.15 0.15 0.15 0.5] Call when an Enemy Dies to clear space for more Enemies to Spawn
  (Math|Integer|DecrementInt (Variables|VariableData|GetSpawnedEnemies)))

(event EventBeginPlay
  ;[0.15 0.15 0.15 0.5] System Initialization (Setting up Data and Correct Values)
  (Initialization|SetSettingsData)
  (Initialization|SetWavesData)
  (Initialization|ClampValues)
  ;[0.15 0.15 0.15 0.5] Initiate Spawn Loop
  (CallFunction|SpawnEnemiesLoop))

(fn ConstructionScript)

(fn SetSettingsData
  ;[0.15 0.15 0.15 0.5] Get Settings Data from Data Table
  (bind _returnvalue (Utilities|GetDataTableRow "/Game/SSS/DataTables/SSS_DT_Settings.SSS_DT_Settings" (.RowName (Utilities|Struct|BreakDataTableRowHandle (Variables|IDs|GetSettingsID))))
    (:then
      (Variables|StaticData|SetSettings _returnvalue))))

(fn SetWavesData
  ;[0.15 0.15 0.15 0.5] Get Wave Data from Data Table
  (bind _returnvalue (Utilities|GetDataTableRow "/Game/SSS/DataTables/SSS_DT_Waves.SSS_DT_Waves" (.RowName (Utilities|Struct|BreakDataTableRowHandle (Variables|IDs|GetWavesID))))
    (:then
      (Variables|StaticData|SetWavesData _returnvalue))))

(fn ClampValues
  (bind _settings (Variables|StaticData|GetSettings))
  (bind _settings_2 (Variables|StaticData|GetSettings))
  (bind (_spawndistancemin _spawndistancemax) (Utilities|Struct|BreakSSS_S_Settings _settings_2))
  (bind _spawninterval (Utilities|Struct|BreakSSS_S_Settings _settings))
  ;[0.15 0.15 0.15 0.5] Clamp Values to make sure nothing breaks
  (Utilities|Struct|SetmembersinSSS_S_Settings (Variables|StaticData|GetSettings) (Math|Float|Clamp(Float) _spawninterval 0.2 _spawninterval))
  (Utilities|Struct|SetmembersinSSS_S_Settings (Variables|StaticData|GetSettings) (Math|Float|Clamp(Float) _spawndistancemin 0.0 _spawndistancemax) (Math|Float|Clamp(Float) _spawndistancemax _spawndistancemin _spawndistancemax)))

(fn SpawnEnemies
  ;[0.15 0.15 0.15 0.5] Main System Spawn Function
  ;;[0.15 0.15 0.15 0.5] Save a Reference of Player Character
  (LocalVariables|SetTarget (Game|GetPlayerCharacter 0))
  ;;[0.15 0.15 0.15 0.5] Loop Function for every Enemy Data
  (for _array_element (Utilities|Struct|BreakSSS_S_WaveData (Utilities|Array|Get(acopy) (Utilities|Struct|BreakSSS_S_WavesData (Variables|StaticData|GetWavesData)) (Variables|VariableData|GetCurrentWave)))
    ;;[0.15 0.15 0.15 0.5] Save a Reference of Enemy Spawn Data
    (LocalVariables|SetEnemyData _array_element)
    ;;[0.15 0.15 0.15 0.5] Check for Enemy Limit before trying to Spawn more
    (if (< (Variables|VariableData|GetSpawnedEnemies) (Utilities|Struct|BreakSSS_S_Settings (Variables|StaticData|GetSettings)))
      ;;[0.15 0.15 0.15 0.5] Enemy Spawn Chance
      (if (Math|Random|RandomBoolwithWeight (Utilities|Struct|BreakSSS_S_WaveIndexData (LocalVariables|GetEnemyData)))
        ;;[0.15 0.15 0.15 0.5] Random Copies of the same enemy to Spawn, from Spawn MIN to Spawn MAX
        (LocalVariables|SetSpawnAmount (Math|Random|RandomIntegerinRange (Math|Integer|Clamp(Integer) (.SpawnMIN (Utilities|Struct|BreakSSS_S_WaveIndexData (LocalVariables|GetEnemyData))) 0 (.SpawnMAX (Utilities|Struct|BreakSSS_S_WaveIndexData (LocalVariables|GetEnemyData)))) (Math|Integer|Clamp(Integer) (.SpawnMAX (Utilities|Struct|BreakSSS_S_WaveIndexData (LocalVariables|GetEnemyData))) (.SpawnMIN (Utilities|Struct|BreakSSS_S_WaveIndexData (LocalVariables|GetEnemyData))) (Utilities|Struct|BreakSSS_S_Settings (Variables|StaticData|GetSettings)))))
        ;;[0.15 0.15 0.15 0.5] Loop Spawn Function base on Amount of Copies
        (for _index (range 0 (- (LocalVariables|GetSpawnAmount) 1))
          ;;[0.15 0.15 0.15 0.5] Check for Enemy Limit before trying to Spawn more
          (if (< (Variables|VariableData|GetSpawnedEnemies) (Utilities|Struct|BreakSSS_S_Settings (Variables|StaticData|GetSettings)))
            ;;[0.15 0.15 0.15 0.5] Find and choose a Random Valid Position if any
            (bind (_found _randomlocation) (SpawnSubFunctions|FindRandomLocation (LocalVariables|GetTarget)))
            (if _found
              (LocalVariables|SetSpawnLocation _randomlocation)
              ;;[0.15 0.15 0.15 0.5] Spawn the Enemy
              (Game|SpawnActorfromClass (.Class (Utilities|Struct|BreakSSS_S_WaveIndexData (LocalVariables|GetEnemyData))) (Math|Transform|MakeTransform (+ (LocalVariables|GetSpawnLocation) (Math|Vector|MakeVector 0.0 0.0 (.CapsuleHalfHeight (Utilities|Struct|BreakSSS_S_WaveIndexData (LocalVariables|GetEnemyData))))) (Math|Rotator|MakeRotator 0.0 0.0 (.yaw (Math|Rotator|FindLookatRotation (LocalVariables|GetSpawnLocation) (Transformation|GetActorLocation (LocalVariables|GetTarget))))) "1.000000,1.000000,1.000000") "AdjustIfPossibleButDontSpawnIfColliding" "MultiplyWithRoot" 0 0)
              ;;[0.15 0.15 0.15 0.5] Increment the Enemy Count
              (Math|Integer|IncrementInt (Variables|VariableData|GetSpawnedEnemies)))))))))

(fn FindRandomLocation
  (params (Target :type Actor%20Object%20Reference))
  (bind _settings (Variables|StaticData|GetSettings))
  (bind _settings_2 (Variables|StaticData|GetSettings))
  (bind _settings_3 (Variables|StaticData|GetSettings))
  (bind _settings_4 (Variables|StaticData|GetSettings))
  (bind _settings_5 (Variables|StaticData|GetSettings))
  (bind _settings_6 (Variables|StaticData|GetSettings))
  (bind _settings_7 (Variables|StaticData|GetSettings))
  (bind (_spawndistancemin _spawndistancemax) (Utilities|Struct|BreakSSS_S_Settings _settings))
  (bind _spawnheightlimit (Utilities|Struct|BreakSSS_S_Settings _settings_4))
  (bind (_spawndistancemin_2 _spawndistancemax_2) (Utilities|Struct|BreakSSS_S_Settings _settings_5))
  (bind _centralspawnheightdistance (Utilities|Struct|BreakSSS_S_Settings _settings_6))
  (bind _spawndistancemin_3 (Utilities|Struct|BreakSSS_S_Settings _settings_7))
  (bind (_usetagsystem _tag) (Utilities|Struct|BreakSSS_S_Settings _settings_2))
  (bind _centralspawnheightdistance_2 (Utilities|Struct|BreakSSS_S_Settings _settings_3))
  (bind _returnvalue (Transformation|GetActorLocation Target))
  (bind _returnvalue_2 (Transformation|GetActorLocation Target))
  (bind _returnvalue_3 (+ _centralspawnheightdistance _spawndistancemin_3))
  ;[0.15 0.15 0.15 0.5] Make a ring around the Player Character using Spawn Distance MIN and Spawn Distance MAX, then choose a Random Valid Position to Spawn an Enemy
  ;;[0.15 0.15 0.15 0.5] Find the Radius
  (LocalVariables|SetRadius (/ (- _spawndistancemax _spawndistancemin) 2.0))
  ;;[0.15 0.15 0.15 0.5] Find the ring's Distance from the Player Character
  (LocalVariables|SetDistance (+ (Utilities|Struct|BreakSSS_S_Settings (Variables|StaticData|GetSettings)) (LocalVariables|GetRadius)))
  ;;[0.15 0.15 0.15 0.5] Find the Amount of Spheres that can fill the ring
  (LocalVariables|SetAmount (Math|Float|Ceil (/ (* (LocalVariables|GetDistance) 3.14 2.0) (- _spawndistancemax_2 _spawndistancemin_2))))
  ;;[0.15 0.15 0.15 0.5] Find and validate possible central spawn positions, if Central Spawn is True
  (if (Utilities|Struct|BreakSSS_S_Settings (Variables|StaticData|GetSettings))
    (for _index (range 0 1)
      (LocalVariables|SetCentralHeight (Utilities|Select :Index _index :Option%200 (+ _returnvalue_2 (Math|Vector|MakeVector 0.0 0.0 _returnvalue_3)) :Option%201 (- _returnvalue_2 (Math|Vector|MakeVector 0.0 0.0 _returnvalue_3))))
      (if (Utilities|Struct|BreakSSS_S_Settings (Variables|StaticData|GetSettings))
        (Collision|SphereTraceByChannel (LocalVariables|GetCentralHeight) (LocalVariables|GetCentralHeight) (Utilities|Struct|BreakSSS_S_Settings (Variables|StaticData|GetSettings)) "TraceTypeQuery1" false 0 "ForDuration" true "(R=1.000000,G=0.885502,B=0.000000,A=1.000000)" "(R=1.000000,G=0.885502,B=0.000000,A=1.000000)" (Utilities|Struct|BreakSSS_S_Settings (Variables|StaticData|GetSettings))))
      (bind (_randomlocation _returnvalue_4) (Class|NavigationSystemV1|GetRandomLocationinNavigableRadius (LocalVariables|GetCentralHeight) (Utilities|Struct|BreakSSS_S_Settings (Variables|StaticData|GetSettings)) 0 0))
      (if _returnvalue_4
        (if (Utilities|Select :Index _index :Option%200 (>= (.Z (Math|Vector|BreakVector _randomlocation)) (+ (.z _returnvalue) _centralspawnheightdistance_2)) :Option%201 (<= (.Z (Math|Vector|BreakVector _randomlocation)) (- (.z _returnvalue) _centralspawnheightdistance_2)))
          (Utilities|Array|Add (LocalVariables|GetPossibleLocations) _randomlocation)))))
  ;;[0.15 0.15 0.15 0.5] Fill the ring with Spheres to find Valid Random Spawn Positions
  (for _index_2 (range 0 (LocalVariables|GetAmount))
    (Utilities|Array|Clear (LocalVariables|GetPossibleHeights))
    (LocalVariables|SetComparing false)
    (LocalVariables|SetOptimalDistance 0.0)
    (LocalVariables|SetOptimalHeight "0, 0, 0")
    (bind _outhits (Collision|MultiSphereTraceForObjects (+ (+ (Transformation|GetActorLocation Target) (* (Math|Vector|GetForwardVector (Math|Rotator|MakeRotator 0.0 0.0 (* (/ 360 (LocalVariables|GetAmount)) _index_2))) (LocalVariables|GetDistance))) (Math|Vector|MakeVector 0.0 0.0 _spawnheightlimit)) (- (+ (Transformation|GetActorLocation Target) (* (Math|Vector|GetForwardVector (Math|Rotator|MakeRotator 0.0 0.0 (* (/ 360 (LocalVariables|GetAmount)) _index_2))) (LocalVariables|GetDistance))) (Math|Vector|MakeVector 0.0 0.0 _spawnheightlimit)) (LocalVariables|GetRadius) (Utilities|Array|MakeArray "ObjectTypeQuery1" "ObjectTypeQuery2") false (Utilities|Array|MakeArray (Game|GetPlayerCharacter 0)) (select (Utilities|Struct|BreakSSS_S_Settings (Variables|StaticData|GetSettings)) "ForDuration" "None") true "(R=0.000000,G=0.105791,B=1.000000,A=1.000000)" "(R=0.220391,G=1.000000,B=0.000000,A=1.000000)" (Utilities|Struct|BreakSSS_S_Settings (Variables|StaticData|GetSettings))))
    (for _array_element _outhits
      (Utilities|IsValid (.HitActor (Collision|BreakHitResult _array_element))
        (:Is%20Valid
          (if _usetagsystem
            (if (Actor|ActorHasTag (.HitActor (Collision|BreakHitResult _array_element)) _tag)
              (Utilities|Array|Add (LocalVariables|GetPossibleHeights) (Math|Vector|MakeVector (.X (Math|Vector|BreakVector (.Location (Collision|BreakHitResult _array_element)))) (.Y (Math|Vector|BreakVector (.Location (Collision|BreakHitResult _array_element)))) (.Z (Math|Vector|BreakVector (.ImpactPoint (Collision|BreakHitResult _array_element))))) :!label _label)
              (else
                (Utilities|IsValid (.HitComponent (Collision|BreakHitResult _array_element))
                  (:Is%20Valid
                    (if (Components|ComponentHasTag (.HitComponent (Collision|BreakHitResult _array_element)) _tag)
                      (goto _label))))))
            (else
              (goto _label))))))
    ;;[0.15 0.15 0.15 0.5] Choose Closets Height Position
    (if (Utilities|Array|IsNotEmpty (LocalVariables|GetPossibleHeights))
      (if (Utilities|Struct|BreakSSS_S_Settings (Variables|StaticData|GetSettings))
        (if (> (Utilities|Array|Length (LocalVariables|GetPossibleHeights)) 1)
          (for _array_element_2 (LocalVariables|GetPossibleHeights)
            (if (LocalVariables|GetComparing)
              (if (< (Math|Float|Absolute(Float) (- (.Z (Math|Vector|BreakVector _array_element_2)) (.z (Transformation|GetActorLocation Target)))) (LocalVariables|GetOptimalDistance))
                (LocalVariables|SetOptimalDistance (Math|Float|Absolute(Float) (- (.Z (Math|Vector|BreakVector _array_element_2)) (.z (Transformation|GetActorLocation Target)))) :!label _label_2)
                (LocalVariables|SetOptimalHeight _array_element_2))
              (else
                (LocalVariables|SetComparing true)
                (goto _label_2))))
          (else
            (LocalVariables|SetOptimalHeight (Utilities|Array|Get(acopy) (LocalVariables|GetPossibleHeights)))))
        (else
          (Utilities|Array|Shuffle (LocalVariables|GetPossibleHeights))
          (LocalVariables|SetOptimalHeight (.OutItem (Utilities|Array|Random (LocalVariables|GetPossibleHeights))))))
      (if (Utilities|Struct|BreakSSS_S_Settings (Variables|StaticData|GetSettings))
        (Collision|SphereTraceByChannel (LocalVariables|GetOptimalHeight) (LocalVariables|GetOptimalHeight) (LocalVariables|GetRadius) "TraceTypeQuery1" false 0 "ForDuration" true "(R=1.000000,G=0.885502,B=0.000000,A=1.000000)" "(R=1.000000,G=0.885502,B=0.000000,A=1.000000)" (Utilities|Struct|BreakSSS_S_Settings (Variables|StaticData|GetSettings))))
      (bind (_randomlocation_2 _returnvalue_5) (Class|NavigationSystemV1|GetRandomLocationinNavigableRadius (LocalVariables|GetOptimalHeight) (LocalVariables|GetRadius) 0 0))
      (if _returnvalue_5
        (if (Utilities|Operators|EqualEqual _randomlocation_2 (LocalVariables|GetOptimalHeight) (LocalVariables|GetRadius))
          (Utilities|Array|Add (LocalVariables|GetPossibleLocations) _randomlocation_2)))))
  ;;[0.15 0.15 0.15 0.5] Choose a Random Position if any
  (if (Utilities|Array|IsNotEmpty (LocalVariables|GetPossibleLocations))
    (Utilities|Array|Shuffle (LocalVariables|GetPossibleLocations))
    (return true (.OutItem (Utilities|Array|Random (LocalVariables|GetPossibleLocations))))
    (else
      (return false "0, 0, 0"))))